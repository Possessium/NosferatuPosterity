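; BP_Grabeable is a base actor for objects that fly toward a player once grabbed.
; Grab stores the player as the target and flags the actor, so Tick moves it toward that target at Speed, scaled by delta time and without sweep.
; Within DistanceGrabbed it calls Grabbed, an empty function here, then destroys itself.
; BeginPlay caches BP_GameState, which these graphs do not otherwise use.
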(event `self.ReceiveBeginPlay`
  (set `self.GameState` (cast `/Game/Blueprints/GameManager/BP_GameState` (`GameplayStatics.GetGameState`) :!pure true)))

(event `self.ReceiveTick`
  (params (DeltaSeconds :type "Float (single-precision)"))
  ;[1 0.964 0.4597] Goes towards the player if grabbed
  (if (`self.IsGrabbed`)
    (`self.K2_SetActorLocation` (+ (`self.K2_GetActorLocation`) (* (`KismetMathLibrary.Normal` (`KismetMathLibrary.GetDirectionUnitVector` (`self.K2_GetActorLocation`) (`self.K2_GetActorLocation` (`self.Target`)))) (* (`GameplayStatics.GetWorldDeltaSeconds`) (`self.Speed`)))))
    (if (< (`self.GetDistanceTo` (`self.Target`)) (`self.DistanceGrabbed`))
      (`self.Grabbed`)
      (`self.K2_DestroyActor`))))

(fn `Grab`
  (params (Player :type "/Game/Blueprints/Characters/Player/BP_Player Object Reference"))
  (set `self.Target` Player)
  (set `self.IsGrabbed` true))

(fn `Grabbed`)

(fn `UserConstructionScript`)