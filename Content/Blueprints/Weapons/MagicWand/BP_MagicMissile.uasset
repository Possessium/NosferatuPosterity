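; BP_MagicMissile is a magic wand projectile that damages the actor it overlaps.
; On BeginPlay it sets its ProjectileMovement velocity along the actor's forward vector, scaled by a Velocity variable.
; A StaticMesh overlap applies Damages to the other actor and destroys the missile, with no filtering of what it hits.
; Tick accumulates elapsed time to destroy the missile after a few seconds, instead of using a lifespan or timer.
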(event `self.ReceiveTick`
  (params (DeltaSeconds :type "Float (single-precision)"))
  (bind _output_get (set `self.Duration` (+ DeltaSeconds (`self.Duration`))))
  (if (>= _output_get 3.0)
    (`self.K2_DestroyActor`)))

(event `self.ReceiveBeginPlay`
  (bind _velocity (`self.Velocity`))
  (set `MovementComponent.Velocity` (* (`KismetMathLibrary.GetForwardVector` (`self.K2_GetActorRotation`)) (`KismetMathLibrary.MakeVector` _velocity _velocity _velocity)) (`self.ProjectileMovement`)))

(event `self.StaticMesh.OnComponentBeginOverlap`
  (params (OverlappedComponent :type "PrimitiveComponent Object Reference") (OtherActor :type "Actor Object Reference") (OtherComp :type "PrimitiveComponent Object Reference") (OtherBodyIndex :type Integer) (bFromSweep :type Boolean) (SweepResult :type "HitResult Structure (by ref)"))
  (`GameplayStatics.ApplyDamage` OtherActor (`self.Damages`))
  (`self.K2_DestroyActor`))

(fn `UserConstructionScript`)