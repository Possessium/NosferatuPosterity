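; BP_SpawnBreakable is a spawn point that randomly places a BP_Breakable at its own location.
; SpawnBreakable rolls against SpawnChance when IsObjectSpawned is false, then spawns the breakable, passes itself as SpawnBreakableOwner and sets the flag.
; ResetObjectSpawned clears that flag to allow another spawn; neither function is called within this Blueprint.
; A leftover "Hello" debug print runs on every SpawnBreakable call.
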(fn `ResetObjectSpawned`
  (set `self.IsObjectSpawned` false))

(fn `SpawnBreakable`
  (`KismetSystemLibrary.PrintString` "Hello")
  (if (`self.IsObjectSpawned`)
    _
    (elif (<= (`KismetMathLibrary.RandomFloatInRange` 0.0 100.0) (`self.SpawnChance`))
      (bind _returnvalue (`|SpawnActorFromClass` "/Game/Blueprints/Breakable/BP_Breakable.BP_Breakable_C" (`KismetMathLibrary.MakeTransform` (`self.K2_GetActorLocation`)) "Undefined" "OverrideRootScale" null null))
      (set `/Game/Blueprints/Breakable/BP_Breakable.SpawnBreakableOwner` self _returnvalue)
      (set `self.IsObjectSpawned` true))))

(fn `UserConstructionScript`)