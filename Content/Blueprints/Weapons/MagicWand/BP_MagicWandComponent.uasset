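; Magic Wand weapon component that extends a parent attack by spawning projectiles from the player toward the nearest enemies.
; GetNearbyEnemies insertion-sorts every BP_Enemy in the level by distance to the owner, with no range limit.
; Attack loops over Quantity, aiming each spawn at the matching enemy's capsule, or firing a BP_MagicMissile at random yaw when none exists.
; Debug prints show each chosen target.
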(fn `Attack`
  (bind (_returnvalue_location _returnvalue_rotation _returnvalue_scale) (`KismetMathLibrary.BreakTransform` (`Actor.GetTransform` (`GameplayStatics.GetPlayerPawn` 0))))
  (bind (_returnvalue_location_2 _returnvalue_rotation_2 _returnvalue_scale_2) (`KismetMathLibrary.BreakTransform` (`Actor.GetTransform` (`GameplayStatics.GetPlayerPawn` 0))))
  (`parent.Attack`)
  (bind _sortedenemies (`self.GetNearbyEnemies`))
  (for _index (range (+ (`self.Quantity`) 1))
    (bind _output (`|GetArrayItem` _sortedenemies _index))
    (`/Engine/EditorBlueprintResources/StandardMacros.IsValid` _output
      (:`Is Valid`
        (`KismetSystemLibrary.PrintString` (`KismetSystemLibrary.GetDisplayName` _output))
        (`|SpawnActorFromClass` "/Game/Blueprints/Weapons/MagicWand/BP_MagicMissile.BP_MagicMissile_C" (`KismetMathLibrary.MakeTransform` _returnvalue_location_2 (`KismetMathLibrary.Conv_VectorToRotator` (`KismetMathLibrary.GetDirectionUnitVector` _returnvalue_location_2 (`SceneComponent.K2_GetComponentLocation` (`Character.CapsuleComponent` _output)))) _returnvalue_scale_2) "Undefined" "OverrideRootScale" null null))
      (:`Is Not Valid`
        (`KismetSystemLibrary.PrintString` "None")
        (`|SpawnActorFromClass` "/Game/Blueprints/Weapons/MagicWand/BP_MagicMissile.BP_MagicMissile_C" (`KismetMathLibrary.MakeTransform` _returnvalue_location (`KismetMathLibrary.MakeRotator` 0.0 0.0 (`KismetMathLibrary.RandomFloatInRange` 0.0 360.0)) _returnvalue_scale) "Undefined" "OverrideRootScale" null null)))))

(fn `GetNearbyEnemies`
  (returns (SortedEnemies :type "Array of /Game/Blueprints/Enemies/BP_Enemy Object Reference"))
  (bind _currenttargetcheckedindex (`self.CurrentTargetCheckedIndex`))
  (`KismetArrayLibrary.Array_Clear` (`self.SortedEnemies`))
  (bind _outactors (`GameplayStatics.GetAllActorsOfClass` "/Game/Blueprints/Enemies/BP_Enemy.BP_Enemy_C"))
  (for (_array_element _array_index) _outactors
    (set `self.CurrentTargetChecked` _array_element)
    (set `self.CurrentTargetCheckedIndex` _array_index)
    (set `self.CurrentTargetDistance` (`Actor.GetDistanceTo` (`self.GetOwner`) (`self.CurrentTargetChecked`)))
    (while (and (> (`Actor.GetDistanceTo` (`self.GetOwner`) (`|GetArrayItem` (`self.SortedEnemies`) (- _currenttargetcheckedindex 1))) (`self.CurrentTargetDistance`)) (> _currenttargetcheckedindex 0))
      (`/Engine/EditorBlueprintResources/StandardMacros.DecrementInt` (`self.CurrentTargetCheckedIndex`)))
    (`KismetArrayLibrary.Array_Insert` (`self.SortedEnemies`) (`self.CurrentTargetChecked`) (`self.CurrentTargetCheckedIndex`)))
  (return (`self.SortedEnemies`)))