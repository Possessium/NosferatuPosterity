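; BP_Player is the player character, handling axis movement, health, timed post-hit invulnerability and XP leveling.
; On start it grants one of three random items via GameState, which also supplies tuning values and handles XP and level-up calls.
; Each tick a sphere overlap grabs nearby BP_Grabeable actors, with debug shapes drawn.
; A viewport-sized detection box triggers BP_SpawnBreakable spawners it begins overlapping.
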(event `InputAxis|MoveXKeyboard`
  (params (AxisValue :type "Float (single-precision)"))
  ;[0.3719 1 0.9402] Controls
  (`self.Input` (`KismetMathLibrary.MakeVector` 0.0 AxisValue)))

(event `InputAxis|MoveYKeyboard`
  (params (AxisValue :type "Float (single-precision)"))
  ;[0.3719 1 0.9402] Controls
  (`self.Input` (`KismetMathLibrary.MakeVector` AxisValue)))

(event `InputAxis|MoveYGamePad`
  (params (AxisValue :type "Float (single-precision)"))
  ;[0.3719 1 0.9402] Controls
  (`self.Input` (`KismetMathLibrary.MakeVector` AxisValue)))

(event `InputAxis|MoveXGamepad`
  (params (AxisValue :type "Float (single-precision)"))
  ;[0.3719 1 0.9402] Controls
  (`self.Input` (`KismetMathLibrary.MakeVector` 0.0 AxisValue)))

(event `self.ReceiveBeginPlay`
  (bind (_returnvalue_x _returnvalue_y) (`KismetMathLibrary.BreakVector2D` (`WidgetLayoutLibrary.GetViewportSize`)))
  (`parent.ReceiveBeginPlay`)
  (set `self.Health` (`/Game/Blueprints/GameManager/BP_GameState.PlayerMaxHealth` (`self.GameState`)))
  (`self.UpdateHealthVisual`)
  (`BoxComponent.SetBoxExtent` (`self.BreakableDetection`) (`KismetMathLibrary.MakeVector` _returnvalue_y _returnvalue_x 50.0) true)
  (`KismetSystemLibrary.Delay` (`KismetMathLibrary.RandomFloatInRange` 0.25 0.5))
  (`/Game/Blueprints/GameManager/BP_GameState.GrabItem` (`self.GameState`) (select `int` (`KismetMathLibrary.RandomInteger` 3) :`0` "NewEnumerator0" :`1` "NewEnumerator1" :`2` "NewEnumerator2" :!type "/Game/Blueprints/EGrabeableItems Enum")))

(event `self.ReceiveTick`
  (params (DeltaSeconds :type "Float (single-precision)"))
  (bind (_returnvalue_x _returnvalue_y) (`KismetMathLibrary.BreakVector2D` (`WidgetLayoutLibrary.GetViewportSize`)))
  (`KismetSystemLibrary.DrawDebugBox` (`self.K2_GetActorLocation`) (`KismetMathLibrary.MakeVector` _returnvalue_y _returnvalue_x 50.0) (struct :`R` 1.0 :`B` 0.007289 :`A` 1.0) (struct) 0.0 5.0)
  (`self.GrabAround`)
  (if (`self.IsInvulnerable`)
    (bind _output_get (set `self.InvulnerabilityTime` (+ DeltaSeconds (`self.InvulnerabilityTime`))))
    (if (>= _output_get (`/Game/Blueprints/GameManager/BP_GameState.InvulnarabilityDuration` (`self.GameState`)))
      (set `self.IsInvulnerable` false)
      (set `self.InvulnerabilityTime` 0.0))))

(event `self.ReceiveAnyDamage`
  (params (Damage :type "Float (single-precision)") (DamageType :type "DamageType Object Reference") (InstigatedBy :type "Controller Object Reference") (DamageCauser :type "Actor Object Reference"))
  (if (not (`self.IsInvulnerable`))
    (`parent.ReceiveAnyDamage` Damage null null null)
    (`self.Hit`)))

(event `self.BreakableDetection.OnComponentBeginOverlap`
  (params (OverlappedComponent :type "PrimitiveComponent Object Reference") (OtherActor :type "Actor Object Reference") (OtherComp :type "PrimitiveComponent Object Reference") (OtherBodyIndex :type Integer) (bFromSweep :type Boolean) (SweepResult :type "HitResult Structure (by ref)"))
  (bind _asbp_spawn_breakable (cast `/Game/Blueprints/Breakable/BP_SpawnBreakable` OtherActor))
  (`/Game/Blueprints/Breakable/BP_SpawnBreakable.SpawnBreakable` _asbp_spawn_breakable))

(fn `AugmentXP`
  (params (Amount :type Integer))
  (bind _gamestate (`self.GameState`))
  (bind _playerlevel (`self.PlayerLevel`))
  (bind _returnvalue (* (+ _playerlevel 1) 5))
  (bind _output_get (set `self.PlayerXP` (+ Amount (`self.PlayerXP`))))
  (`/Game/Blueprints/GameManager/BP_GameState.GetXP` (`self.GameState`) (/ _output_get _returnvalue) _playerlevel)
  (if (>= _output_get _returnvalue)
    (set `self.PlayerXP` (- (`self.PlayerXP`) _returnvalue))
    (bind _result (`/Engine/EditorBlueprintResources/StandardMacros.IncrementInt` (`self.PlayerLevel`))
      (:`  `
        (`/Game/Blueprints/GameManager/BP_GameState.GetXP` _gamestate 0.0 _result)
        (`/Game/Blueprints/GameManager/BP_GameState.LevelupItems` _gamestate)))))

(fn `GrabAround`
  (bind _returnvalue (`self.K2_GetActorLocation`))
  (bind _radiusgrab (`/Game/Blueprints/GameManager/BP_GameState.RadiusGrab` (`self.GameState`)))
  (`KismetSystemLibrary.DrawDebugSphere` _returnvalue _radiusgrab 12 (struct :`R` 1.0 :`B` 0.203858 :`A` 1.0) 0.0 1.0)
  (bind _outactors (`KismetSystemLibrary.SphereOverlapActors` _returnvalue _radiusgrab (`|MakeArray` "ObjectTypeQuery2" :!type "EObjectTypeQuery Enum") "/Game/Blueprints/Grabeable/BP_Grabeable.BP_Grabeable_C"))
  (for _array_element _outactors
    (bind _asbp_grabeable (cast `/Game/Blueprints/Grabeable/BP_Grabeable` _array_element))
    (`/Game/Blueprints/Grabeable/BP_Grabeable.Grab` _asbp_grabeable self)))

(fn `Heal`
  (params (Amount :type "Float (double-precision)"))
  (set `self.Health` (`KismetMathLibrary.FClamp` (+ Amount (`self.Health`)) 0.0 (`/Game/Blueprints/GameManager/BP_GameState.PlayerMaxHealth` (`self.GameState`))))
  (`self.UpdateHealthVisual`))

(fn `Hit`
  (if (not (`self.IsInvulnerable`))
    (`parent.Hit`)
    (set `self.IsInvulnerable` true)))

(fn `Input`
  (params (Direction :type "Vector Structure"))
  (bind (_x _y) (`KismetMathLibrary.BreakVector3f` Direction))
  (`self.AddMovementInput` Direction)
  (if (!= _y 0.0)
    (set `self.IsLookingLeft` (< _y 0.0))))

(fn `UserConstructionScript`)