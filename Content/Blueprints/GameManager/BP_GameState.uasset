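; Game state for a Vampire Survivors-style run, holding weapon and passive item stats, elapsed time, kills and money, and updating the HUD.
; Level-up slows time through eased global dilation and offers three random items, occasionally four.
; GrabItem applies capped percentage upgrades, adds weapon components on first pick and restores time; whip delay reductions multiply by zero, so have no effect.
; SpawnGem rolls red, blue or green XP gems.
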(event `self.ReceiveBeginPlay`
  (set `self.Player` (cast `/Game/Blueprints/Characters/Player/BP_Player` (`GameplayStatics.GetPlayerPawn` 0) :!pure true))
  (bind _returnvalue (`|CreateWidget` "/Game/Blueprints/UI/WBP_LevelUP.WBP_LevelUP_C"))
  (bind _output_get (set `self.WidgetLevelup` _returnvalue))
  (`UserWidget.AddToViewport` _output_get 1)
  (`Widget.SetVisibility` _returnvalue "Hidden")
  (`Widget.SetVisibility` _output_get "Hidden")
  (bind _returnvalue_2 (`|CreateWidget` "/Game/Blueprints/UI/WBP_GameUI.WBP_GameUI_C"))
  (bind _output_get_2 (set `self.GameUI` _returnvalue_2))
  (`UserWidget.AddToViewport` _output_get_2 0))

(event `self.ReceiveTick`
  (params (DeltaSeconds :type "Float (single-precision)"))
  (`|ExecutionSequence`
    (:`then_0`
      (if (`self.GameStarted`)
        (set `self.CurrentElapsedTime` (+ (`self.CurrentElapsedTime`) (* DeltaSeconds (`self.SlowingElapsedTime`))))))
    (:`then_1`
      (`/Game/Blueprints/UI/WBP_GameUI.ChangeTimeValue` (`self.GameUI`) (`KismetMathLibrary.FromSeconds` (`self.CurrentElapsedTime`))))
    (:`then_2`
      (bind _output_get (set `self.SlowingElapsedTime` (`KismetMathLibrary.FClamp` (+ (* DeltaSeconds (`self.TimeChangeSpeed`)) (`self.SlowingElapsedTime`)) 0.15)))
      (if (and (`self.IsSlowingTime`) (< _output_get 1.0))
        (`GameplayStatics.SetGlobalTimeDilation` (`KismetMathLibrary.Lerp` 1.0 0.15 (`self.SlowingElapsedTime`)))
        (elif (and (not (`self.IsSlowingTime`)) (< (`self.SlowingElapsedTime`) 1.0))
          (`GameplayStatics.SetGlobalTimeDilation` (`KismetMathLibrary.Lerp` 0.15 1.0 (`self.SlowingElapsedTime`))))))))

(fn `AddAttractorb`
  (if (< (`self.AttractorbCount`) (`self.MaxAttractorb`))
    (`/Engine/EditorBlueprintResources/StandardMacros.IncrementInt` (`self.AttractorbCount`)
      (:`  `
        (`self.AugmentPlayerRadius` (`self.PlayerRangeAugmentPercent`))))))

(fn `AddChandelier`
  (if (< (`self.ChandelierCount`) (`self.MaxChandelier`))
    (`/Engine/EditorBlueprintResources/StandardMacros.IncrementInt` (`self.ChandelierCount`)
      (:`  `
        (`self.AugmentAllRadius` (`self.ChandelierRangeAugmentPercent`))))))

(fn `AddEmptyTome`
  (if (< (`self.EmptyTomeCount`) (`self.MaxEmptyTome`))
    (`/Engine/EditorBlueprintResources/StandardMacros.IncrementInt` (`self.EmptyTomeCount`)
      (:`  `
        (`self.ReduceAllDelays` (`self.EmptyTomeDelayReducedPercent`))))))

(fn `AddKill`
  (bind _result (`/Engine/EditorBlueprintResources/StandardMacros.IncrementInt` (`self.KillAmount`))
    (:`  `
      (`/Game/Blueprints/UI/WBP_GameUI.ChangeKillValue` (`self.GameUI`) _result))))

(fn `AugmentAllDamages`
  (params (DamageAugmentPercent :type "Float (double-precision)"))
  (bind _whipattackdamage (`self.WhipAttackDamage`))
  (bind _wandattackdamage (`self.WandAttackDamage`))
  (bind _garlicattackdamage (`self.GarlicAttackDamage`))
  (`|ExecutionSequence`
    (:`then_0`
      (set `self.WandAttackDamage` (+ (* _wandattackdamage (/ DamageAugmentPercent 100)) _wandattackdamage)))
    (:`then_1`
      (set `self.WhipAttackDamage` (+ (* _whipattackdamage (/ DamageAugmentPercent 100)) _whipattackdamage)))
    (:`then_2`
      (set `self.GarlicAttackDamage` (+ (* _garlicattackdamage (/ DamageAugmentPercent 100)) _garlicattackdamage)))))

(fn `AugmentAllRadius`
  (params (RadiusAugmentPercent :type "Float (double-precision)"))
  (bind _returnvalue (/ RadiusAugmentPercent 100))
  (bind (_whipattacksize_x _whipattacksize_y) (`KismetMathLibrary.BreakVector` (`self.WhipAttackSize`)))
  (bind _whipattacksize_x_2 (`KismetMathLibrary.BreakVector` (`self.WhipAttackSize`)))
  (bind _wandattackradius (`self.WandAttackRadius`))
  (bind _garlicattackradius (`self.GarlicAttackRadius`))
  (`|ExecutionSequence`
    (:`then_0`
      (set `self.WandAttackRadius` (+ (* _wandattackradius (/ RadiusAugmentPercent 100)) _wandattackradius)))
    (:`then_1`
      (set `self.WhipAttackSize` (`KismetMathLibrary.MakeVector` (+ (* _whipattacksize_x_2 _returnvalue) _whipattacksize_x_2) (+ (* _whipattacksize_y _returnvalue) _whipattacksize_y))))
    (:`then_2`
      (set `self.GarlicAttackRadius` (+ (* _garlicattackradius (/ RadiusAugmentPercent 100)) _garlicattackradius)))))

(fn `AugmentGarlic`
  (bind _garlicattackdelay (`self.GarlicAttackDelay`))
  (bind _garlicattackdamage (`self.GarlicAttackDamage`))
  (bind _garlicattackradius (`self.GarlicAttackRadius`))
  (if (< (`self.GarlicQuantity`) (`self.MaxGarlic`))
    (`/Engine/EditorBlueprintResources/StandardMacros.IncrementInt` (`self.GarlicQuantity`)
      (:`  `
        (`|ExecutionSequence`
          (:`then_0`
            (set `self.GarlicAttackDamage` (+ (* _garlicattackdamage (/ (`self.GarlicAugmentDamageValue`) 100)) _garlicattackdamage)))
          (:`then_1`
            (set `self.GarlicAttackRadius` (+ (* _garlicattackradius (/ (`self.GarlicAugmentRadiusValue`) 100)) _garlicattackradius)))
          (:`then_2`
            (set `self.GarlicAttackDelay` (- _garlicattackdelay (* _garlicattackdelay (/ (`self.GarlicReduceDelayValue`) 100))))))))))

(fn `AugmentMagicWand`
  (bind _wandattackdelay (`self.WandAttackDelay`))
  (bind _wandattackradius (`self.WandAttackRadius`))
  (bind _wandattackdamage (`self.WandAttackDamage`))
  (bind _wandquantity (`self.WandQuantity`))
  (if (< (`self.WandQuantity`) (`self.MaxWand`))
    (`/Engine/EditorBlueprintResources/StandardMacros.IncrementInt` _wandquantity
      (:`  `
        (if (not (<= _wandquantity 1))
          (`|ExecutionSequence`
            (:`then_0`
              (set `self.WandAttackDamage` (+ (* _wandattackdamage (/ (`self.WandAugmentDamageValue`) 100)) _wandattackdamage)))
            (:`then_1`
              (set `self.WandAttackRadius` (+ (* _wandattackradius (/ (`self.WandAugmentRadiusValue`) 100)) _wandattackradius)))
            (:`then_2`
              (set `self.WandAttackDelay` (- _wandattackdelay (* _wandattackdelay (/ (`self.WandReduceDelayValue`) 100)))))))))))

(fn `AugmentPlayerRadius`
  (params (PlayerRangeAugmentPercent :type "Float (double-precision)"))
  (bind _radiusgrab (`self.RadiusGrab`))
  (set `self.RadiusGrab` (+ (* _radiusgrab (/ PlayerRangeAugmentPercent 100.0)) _radiusgrab)))

(fn `AugmentWhip`
  (bind _whipattackdamage (`self.WhipAttackDamage`))
  (bind _whipattackdelay (`self.WhipAttackDelay`))
  (bind (_whipattacksize_x _whipattacksize_y) (`KismetMathLibrary.BreakVector` (`self.WhipAttackSize`)))
  (if (< (`self.WhipQuantity`) (`self.MaxWhip`))
    (`/Engine/EditorBlueprintResources/StandardMacros.IncrementInt` (`self.WhipQuantity`)
      (:`  `
        (`|ExecutionSequence`
          (:`then_0`
            (set `self.WhipAttackDamage` (+ (* _whipattackdamage (/ (`self.WhipAugmentDamageValue`) 100)) _whipattackdamage)))
          (:`then_1`
            (set `self.WhipAttackSize` (`KismetMathLibrary.MakeVector` (+ (* _whipattacksize_x (/ (`self.WhipAugmentRadiusValue`) 100)) _whipattacksize_x) (+ _whipattacksize_y (* _whipattacksize_y (/ (`self.WhipAugmentRadiusValue`) 100))))))
          (:`then_2`
            (set `self.WhipAttackDelay` (- _whipattackdelay (* 0.0 _whipattackdelay)))))))))

(fn `GetXP`
  (params (`XP Percent` :type "Float (double-precision)") (Level :type Integer))
  (`/Game/Blueprints/UI/WBP_GameUI.ChangeXPValue` (`self.GameUI`) Level `XP Percent`))

(fn `GrabItem`
  (params (`Grabbed item` :type "/Game/Blueprints/EGrabeableItems Enum" :default "NewEnumerator6"))
  (bind _player (`self.Player`))
  (bind _playerlevel (`/Game/Blueprints/Characters/Player/BP_Player.PlayerLevel` _player))
  (set `PlayerController.bShowMouseCursor` false (`GameplayStatics.GetPlayerController` 0))
  (`self.TriggerChangeTime` false)
  (`|ExecutionSequence`
    (:`then_0`
      (switch `/Game/Blueprints/EGrabeableItems` `Grabbed item`
        (:`NewEnumerator0`
          (`self.AugmentMagicWand`)
          ;[0.2723 1 0.8394] Add component if first augment
          (if (== (`self.WandQuantity`) 1)
            (`|AddComponentByClass` (`GameplayStatics.GetPlayerController` 0) "/Game/Blueprints/Weapons/MagicWand/BP_MagicWandComponent.BP_MagicWandComponent_C")))
        (:`NewEnumerator1`
          (`self.AugmentGarlic`)
          (if (== (`self.GarlicQuantity`) 1)
            (`|AddComponentByClass` (`GameplayStatics.GetPlayerController` 0) "/Game/Blueprints/Weapons/Garlic/BP_GarlicComponent.BP_GarlicComponent_C")))
        (:`NewEnumerator2`
          (`self.AugmentWhip`)
          (if (== (`self.WhipQuantity`) 1)
            (`|AddComponentByClass` (`GameplayStatics.GetPlayerController` 0) "/Game/Blueprints/Weapons/Whip/BP_WhipComponent.BP_WhipComponent_C")))
        (:`NewEnumerator3`
          (`self.AddChandelier`))
        (:`NewEnumerator4`
          (`self.AddAttractorb`))
        (:`NewEnumerator5`
          (`self.AddEmptyTome`))))
    (:`then_1`
      (`Widget.SetVisibility` (`self.WidgetLevelup`) "Hidden")
      (`/Game/Blueprints/UI/WBP_GameUI.ChangeXPValue` (`self.GameUI`) _playerlevel (/ (`/Game/Blueprints/Characters/Player/BP_Player.PlayerXP` _player) (* (+ _playerlevel 1) 5))))))

(fn `GrabMoney`
  (params (Amount :type Integer))
  (bind _output_get (set `self.PlayerMoney` (+ Amount (`self.PlayerMoney`))))
  (`/Game/Blueprints/UI/WBP_GameUI.ChangeMoneyValue` (`self.GameUI`) _output_get))

(fn `LevelupItems`
  (locals (Item1 :type "/Game/Blueprints/EGrabeableItems Enum") (Item2 :type "/Game/Blueprints/EGrabeableItems Enum") (Item3 :type "/Game/Blueprints/EGrabeableItems Enum") (Item4 :type "/Game/Blueprints/EGrabeableItems Enum"))
  (bind _returnvalue (select `int` (`KismetMathLibrary.RandomInteger` 6) :`0` "NewEnumerator0" :`1` "NewEnumerator1" :`2` "NewEnumerator2" :`3` "NewEnumerator3" :`4` "NewEnumerator4" :`5` "NewEnumerator5" :!type "/Game/Blueprints/EGrabeableItems Enum"))
  (set `PlayerController.bShowMouseCursor` true (`GameplayStatics.GetPlayerController` 0))
  (`self.TriggerChangeTime` true)
  (set `local.Item1` "NewEnumerator6")
  (set `local.Item2` "NewEnumerator6")
  (set `local.Item3` "NewEnumerator6")
  (set `local.Item4` "NewEnumerator6")
  (`|ExecutionSequence`
    (:`then_0`
      (set `local.Item1` _returnvalue)
      (set `local.Item2` _returnvalue)
      (set `local.Item3` _returnvalue))
    (:`then_1`
      (if (<= (`KismetMathLibrary.RandomFloatInRange` 0.0 100.0) 10.0)
        (set `local.Item4` (select `int` (`KismetMathLibrary.RandomInteger` 6) :`0` "NewEnumerator0" :`1` "NewEnumerator1" :`2` "NewEnumerator2" :`3` "NewEnumerator3" :`4` "NewEnumerator4" :`5` "NewEnumerator5" :!type "/Game/Blueprints/EGrabeableItems Enum"))))
    (:`then_2`
      (`/Game/Blueprints/UI/WBP_LevelUP.ActivatePanels` (`self.WidgetLevelup`) (`local.Item1`) (`local.Item2`) (`local.Item3`) (`local.Item4`)))))

(fn `ReduceAllDelays`
  (params (DelayReducedPercent :type "Float (double-precision)"))
  (bind _garlicattackdelay (`self.GarlicAttackDelay`))
  (bind _wandattackdelay (`self.WandAttackDelay`))
  (bind _whipattackdelay (`self.WhipAttackDelay`))
  (`|ExecutionSequence`
    (:`then_0`
      (set `self.WandAttackDelay` (- _wandattackdelay (* _wandattackdelay (/ DelayReducedPercent 100)))))
    (:`then_1`
      (set `self.WhipAttackDelay` (- _whipattackdelay (* 0.0 _whipattackdelay))))
    (:`then_2`
      (set `self.GarlicAttackDelay` (- _garlicattackdelay (* _garlicattackdelay (/ DelayReducedPercent 100)))))))

(fn `SpawnGem`
  (params (Position :type "Vector Structure"))
  (bind _returnvalue (`KismetMathLibrary.RandomFloatInRange` 0.0 100.0))
  (if (<= _returnvalue (`self.RedGemChance`))
    (`|SpawnActorFromClass` "/Game/Blueprints/Grabeable/Gems/BP_GemRed.BP_GemRed_C" (`KismetMathLibrary.MakeTransform` Position) "Undefined" "OverrideRootScale" null null)
    (elif (<= _returnvalue (`self.BlueGemChance`))
      (`|SpawnActorFromClass` "/Game/Blueprints/Grabeable/Gems/BP_GemBlue.BP_GemBlue_C" (`KismetMathLibrary.MakeTransform` Position) "Undefined" "OverrideRootScale" null null)
      (else
        (`|SpawnActorFromClass` "/Game/Blueprints/Grabeable/Gems/BP_GemGreen.BP_GemGreen_C" (`KismetMathLibrary.MakeTransform` Position) "Undefined" "OverrideRootScale" null null)))))

(fn `TriggerChangeTime`
  (params (IsSlowed :type Boolean))
  (set `self.IsSlowingTime` IsSlowed)
  (set `self.SlowingElapsedTime` 0.0))

(fn `UserConstructionScript`)