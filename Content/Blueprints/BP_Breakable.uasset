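; BP_Breakable is a breakable actor that can drop food or money when broken.
; Its Break function flips a coin between a food roll and a money roll, checked against FoodChances or MoneyChances, so it never drops both.
; A successful food roll picks one of nine food Blueprints at random, while money spawns BP_Money.
; Drops spawn at the actor's location, and the actor then destroys itself whatever the result.
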(fn `Break`
  (locals (RandomFoodIndex :type Integer :default 0))
  (bind _returnvalue (`KismetMathLibrary.MakeTransform` (`self.K2_GetActorLocation`)))
  (`|ExecutionSequence`
    (:`then_0`
      (if (== (`KismetMathLibrary.RandomInteger` 2) 0)
        (if (<= (`KismetMathLibrary.RandomFloatInRange` 0.0 100.0) (`self.FoodChances`))
          (switch `int` (`KismetMathLibrary.RandomInteger` 9)
            (:`0`
              (`|SpawnActorFromClass` "/Game/Blueprints/Grabeable/Food/BP_Bread.BP_Bread_C" _returnvalue "Undefined" "OverrideRootScale" null null))
            (:`1`
              (`|SpawnActorFromClass` "/Game/Blueprints/Grabeable/Food/BP_Cabbage.BP_Cabbage_C" _returnvalue "Undefined" "OverrideRootScale" null null))
            (:`2`
              (`|SpawnActorFromClass` "/Game/Blueprints/Grabeable/Food/BP_Donut.BP_Donut_C" _returnvalue "Undefined" "OverrideRootScale" null null))
            (:`3`
              (`|SpawnActorFromClass` "/Game/Blueprints/Grabeable/Food/BP_Mango.BP_Mango_C" _returnvalue "Undefined" "OverrideRootScale" null null))
            (:`4`
              (`|SpawnActorFromClass` "/Game/Blueprints/Grabeable/Food/BP_Muffin.BP_Muffin_C" _returnvalue "Undefined" "OverrideRootScale" null null))
            (:`5`
              (`|SpawnActorFromClass` "/Game/Blueprints/Grabeable/Food/BP_Peach.BP_Peach_C" _returnvalue "Undefined" "OverrideRootScale" null null))
            (:`6`
              (`|SpawnActorFromClass` "/Game/Blueprints/Grabeable/Food/BP_Pineapple.BP_Pineapple_C" _returnvalue "Undefined" "OverrideRootScale" null null))
            (:`7`
              (`|SpawnActorFromClass` "/Game/Blueprints/Grabeable/Food/BP_Pizza.BP_Pizza_C" _returnvalue "Undefined" "OverrideRootScale" null null))
            (:`8`
              (`|SpawnActorFromClass` "/Game/Blueprints/Grabeable/Food/BP_Watermelon.BP_Watermelon_C" _returnvalue "Undefined" "OverrideRootScale" null null))))
        (elif (<= (`KismetMathLibrary.RandomFloatInRange` 0.0 100.0) (`self.MoneyChances`))
          (`|SpawnActorFromClass` "/Game/Blueprints/Grabeable/BP_Money.BP_Money_C" (`KismetMathLibrary.MakeTransform` (`self.K2_GetActorLocation`)) "Undefined" "OverrideRootScale" null null))))
    (:`then_1`
      (`self.K2_DestroyActor`))))

(fn `UserConstructionScript`)