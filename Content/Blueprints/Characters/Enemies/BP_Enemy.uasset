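; BP_Enemy is an enemy character that damages the player and can drop a gem when killed.
; Kill calls the parent logic, rolls against the GameState drop rate to spawn a gem, records the kill and destroys the actor.
; Attack accumulates delta time and, at the GameState attack rate threshold, applies GameState-defined damage to the player pawn.
; The timer is never reset here, and Attack has no range check.
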(fn `Attack`
  (params (DeltaSeconds :type "Float (double-precision)"))
  (locals (AttackDelayTime :type "Float (double-precision)"))
  (bind _output_get (set `local.AttackDelayTime` (+ DeltaSeconds (`local.AttackDelayTime`))))
  (if (>= _output_get (`/Game/Blueprints/GameManager/BP_GameState.EnemyAttackRate` (`self.GameState`)))
    (bind _asbp_player (cast `/Game/Blueprints/Characters/Player/BP_Player` (`GameplayStatics.GetPlayerPawn` 0)))
    (`GameplayStatics.ApplyDamage` _asbp_player (`/Game/Blueprints/GameManager/BP_GameState.EnemyAttackDamage` (`self.GameState`)))))

(fn `Kill`
  (bind _gamestate (`self.GameState`))
  (`parent.Kill`)
  (`|ExecutionSequence`
    (:`then_0`
      (if (<= (`KismetMathLibrary.RandomFloatInRange` 0.0 100.0) (`/Game/Blueprints/GameManager/BP_GameState.EnemyGemDropRate` _gamestate))
        (`/Game/Blueprints/GameManager/BP_GameState.SpawnGem` _gamestate (`self.K2_GetActorLocation`))))
    (:`then_1`
      (`/Game/Blueprints/GameManager/BP_GameState.AddKill` (`self.GameState`))
      (`self.K2_DestroyActor`))))

(fn `UserConstructionScript`)