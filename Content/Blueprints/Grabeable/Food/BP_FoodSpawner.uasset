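; Spawner actor that creates one random food item at a given position for a given owner.
; SpawnRandomFood stores both inputs, then picks one of nine food Blueprints at random.
; Most picks register the owner on the new food and destroy the spawner.
; Bread and Cabbage only spawn: their owner registration and cleanup are disconnected, so the spawner remains.
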(fn `SpawnRandomFood`
  (params (Position :type "Vector Structure") (Owner :type "/Game/Blueprints/Breakable/BP_SpawnBreakable Object Reference"))
  (locals (FoodPosition :type "Vector Structure") (FoodOwner :type "/Game/Blueprints/Breakable/BP_SpawnBreakable Object Reference"))
  (set `local.FoodPosition` Position)
  (set `local.FoodOwner` Owner)
  (switch `int` (`KismetMathLibrary.RandomInteger` 9)
    (:`0`
      (`|SpawnActorFromClass` "/Game/Blueprints/Grabeable/Food/BP_Bread.BP_Bread_C" (`KismetMathLibrary.MakeTransform` (`local.FoodPosition`)) "Undefined" "OverrideRootScale" null null))
    (:`1`
      (`|SpawnActorFromClass` "/Game/Blueprints/Grabeable/Food/BP_Cabbage.BP_Cabbage_C" (`KismetMathLibrary.MakeTransform` (`local.FoodPosition`)) "Undefined" "OverrideRootScale" null null))
    (:`2`
      (bind _returnvalue (`|SpawnActorFromClass` "/Game/Blueprints/Grabeable/Food/BP_Donut.BP_Donut_C" (`KismetMathLibrary.MakeTransform` (`local.FoodPosition`)) "Undefined" "OverrideRootScale" null null))
      (`/Game/Blueprints/Grabeable/BP_Grabeable.RegisterOwner` _returnvalue (`local.FoodOwner`))
      (`self.K2_DestroyActor` :!label _label))
    (:`3`
      (bind _returnvalue_2 (`|SpawnActorFromClass` "/Game/Blueprints/Grabeable/Food/BP_Mango.BP_Mango_C" (`KismetMathLibrary.MakeTransform` (`local.FoodPosition`)) "Undefined" "OverrideRootScale" null null))
      (`/Game/Blueprints/Grabeable/BP_Grabeable.RegisterOwner` _returnvalue_2 (`local.FoodOwner`))
      (goto _label))
    (:`4`
      (bind _returnvalue_3 (`|SpawnActorFromClass` "/Game/Blueprints/Grabeable/Food/BP_Muffin.BP_Muffin_C" (`KismetMathLibrary.MakeTransform` (`local.FoodPosition`)) "Undefined" "OverrideRootScale" null null))
      (`/Game/Blueprints/Grabeable/BP_Grabeable.RegisterOwner` _returnvalue_3 (`local.FoodOwner`))
      (goto _label))
    (:`5`
      (bind _returnvalue_4 (`|SpawnActorFromClass` "/Game/Blueprints/Grabeable/Food/BP_Peach.BP_Peach_C" (`KismetMathLibrary.MakeTransform` (`local.FoodPosition`)) "Undefined" "OverrideRootScale" null null))
      (`/Game/Blueprints/Grabeable/BP_Grabeable.RegisterOwner` _returnvalue_4 (`local.FoodOwner`))
      (goto _label))
    (:`6`
      (bind _returnvalue_5 (`|SpawnActorFromClass` "/Game/Blueprints/Grabeable/Food/BP_Pineapple.BP_Pineapple_C" (`KismetMathLibrary.MakeTransform` (`local.FoodPosition`)) "Undefined" "OverrideRootScale" null null))
      (`/Game/Blueprints/Grabeable/BP_Grabeable.RegisterOwner` _returnvalue_5 (`local.FoodOwner`))
      (goto _label))
    (:`7`
      (bind _returnvalue_6 (`|SpawnActorFromClass` "/Game/Blueprints/Grabeable/Food/BP_Pizza.BP_Pizza_C" (`KismetMathLibrary.MakeTransform` (`local.FoodPosition`)) "Undefined" "OverrideRootScale" null null))
      (`/Game/Blueprints/Grabeable/BP_Grabeable.RegisterOwner` _returnvalue_6 (`local.FoodOwner`))
      (goto _label))
    (:`8`
      (bind _returnvalue_7 (`|SpawnActorFromClass` "/Game/Blueprints/Grabeable/Food/BP_Watermelon.BP_Watermelon_C" (`KismetMathLibrary.MakeTransform` (`local.FoodPosition`)) "Undefined" "OverrideRootScale" null null))
      (`/Game/Blueprints/Grabeable/BP_Grabeable.RegisterOwner` _returnvalue_7 (`local.FoodOwner`))
      (goto _label))))

(fn `UserConstructionScript`)