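; BP_Money is a grabbable money pickup that awards a random amount of money when grabbed.
; On BeginPlay it rolls MoneyAmount between MinMoneyAmount and MaxMoneyAmount, so each instance's value is fixed at spawn.
; Its Grabbed override runs the parent logic, then passes that amount to GrabMoney on the GameState.
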(event `self.ReceiveBeginPlay`
  (`parent.ReceiveBeginPlay`)
  (set `self.MoneyAmount` (`KismetMathLibrary.RandomIntegerInRange` (`self.MinMoneyAmount`) (`self.MaxMoneyAmount`))))

(fn `Grabbed`
  (`parent.Grabbed`)
  (`/Game/Blueprints/GameManager/BP_GameState.GrabMoney` (`self.GameState`) (`self.MoneyAmount`)))

(fn `UserConstructionScript`
  (`parent.UserConstructionScript`))