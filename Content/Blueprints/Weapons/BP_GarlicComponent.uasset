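; Garlic weapon component that damages every enemy around its owner in an area attack.
; On BeginPlay it takes its attack delay from the GameState's garlic setting.
; Its Attack override calls the parent, runs a sphere overlap at the owner's location filtered to BP_Enemy pawns, and calls Hit on each with garlic damage.
; Radius and damage are read from GameState on each attack.
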(event `self.ReceiveBeginPlay`
  (`parent.ReceiveBeginPlay`)
  (set `self.AttackDelay` (`/Game/Blueprints/GameManager/BP_GameState.GarlicAttackDelay` (`self.GameState`))))

(fn `Attack`
  (`parent.Attack`)
  (bind _outactors (`KismetSystemLibrary.SphereOverlapActors` (`Actor.K2_GetActorLocation` (`self.GetOwner`)) (`/Game/Blueprints/GameManager/BP_GameState.GarlicAttackRadius` (`self.GameState`)) (`|MakeArray` "ObjectTypeQuery3" :!type "EObjectTypeQuery Enum") "/Game/Blueprints/Enemies/BP_Enemy.BP_Enemy_C"))
  (for _array_element _outactors
    (bind _asbp_enemy (cast `/Game/Blueprints/Enemies/BP_Enemy` _array_element))
    (`/Game/Blueprints/Enemies/BP_Enemy.Hit` _asbp_enemy (`/Game/Blueprints/GameManager/BP_GameState.GarlicAttackDamage` (`self.GameState`)))))