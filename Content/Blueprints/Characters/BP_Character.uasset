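; BP_Character is a character Blueprint with health that takes damage and shows its value on a Text3D component.
; BeginPlay caches BP_GameState and refreshes the health text, while Tick holds the text at a fixed world rotation, pitched -90 degrees.
; AnyDamage subtracts from Health, then either updates the text or calls Kill at zero or below.
; Kill and Hit are empty functions here.
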(event `self.ReceiveBeginPlay`
  (bind _asbp_game_state (cast `/Game/Blueprints/GameManager/BP_GameState` (`GameplayStatics.GetGameState`)))
  (set `self.GameState` _asbp_game_state)
  (`self.UpdateHealthVisual`))

(event `self.ReceiveTick`
  (params (DeltaSeconds :type "Float (single-precision)"))
  (`SceneComponent.K2_SetWorldRotation` (`self.Text3D`) (`KismetMathLibrary.MakeRotator` 0.0 -90.0) false false))

(event `self.ReceiveAnyDamage`
  (params (Damage :type "Float (single-precision)") (DamageType :type "DamageType Object Reference") (InstigatedBy :type "Controller Object Reference") (DamageCauser :type "Actor Object Reference"))
  (bind _output_get (set `self.Health` (- (`self.Health`) Damage)))
  (if (<= _output_get 0.0)
    (`self.Kill`)
    (else
      (`self.UpdateHealthVisual`))))

(fn `Hit`)

(fn `Kill`)

(fn `UpdateHealthVisual`
  (`Text3DComponent.SetText` (`self.Text3D`) (`KismetTextLibrary.Conv_DoubleToText` (`self.Health`) "HalfToEven")))

(fn `UserConstructionScript`)