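; BP_Enemy is an enemy actor that shows its health as 3D text and can drop a gem when killed.
; Damage arrives through AnyDamage or the Hit function, which duplicate the same logic to reduce Health, then update the text or call Kill.
; Kill rolls against the EnemyGemDropRate in BP_GameState to spawn BP_Gem, then destroys the actor.
; Tick locks the text to a fixed world rotation.
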(event `self.ReceiveBeginPlay`
  (`Text3DComponent.SetText` (`self.Text3D`) (`KismetTextLibrary.Conv_DoubleToText` (`self.Health`) "HalfToEven"))
  (bind _asbp_game_state (cast `/Game/Blueprints/GameManager/BP_GameState` (`GameplayStatics.GetGameState`)))
  (set `self.GameState` _asbp_game_state))

(event `self.ReceiveTick`
  (params (DeltaSeconds :type "Float (single-precision)"))
  (`SceneComponent.K2_SetWorldRotation` (`self.Text3D`) (`KismetMathLibrary.MakeRotator` 0.0 -90.0) false false))

(event `self.ReceiveAnyDamage`
  (params (Damage :type "Float (single-precision)") (DamageType :type "DamageType Object Reference") (InstigatedBy :type "Controller Object Reference") (DamageCauser :type "Actor Object Reference"))
  (bind _output_get (set `self.Health` (- (`self.Health`) Damage)))
  (if (<= _output_get 0.0)
    (`self.Kill`)
    (else
      (`Text3DComponent.SetText` (`self.Text3D`) (`KismetTextLibrary.Conv_DoubleToText` _output_get "HalfToEven")))))

(fn `Hit`
  (params (Damage :type "Float (double-precision)"))
  (bind _output_get (set `self.Health` (- (`self.Health`) Damage)))
  (if (<= _output_get 0.0)
    (`self.Kill`)
    (else
      (`Text3DComponent.SetText` (`self.Text3D`) (`KismetTextLibrary.Conv_DoubleToText` _output_get "HalfToEven")))))

(fn `Kill`
  (`|ExecutionSequence`
    (:`then_0`
      (if (<= (`KismetMathLibrary.RandomFloatInRange` 0.0 100.0) (`/Game/Blueprints/GameManager/BP_GameState.EnemyGemDropRate` (`self.GameState`)))
        (`|SpawnActorFromClass` "/Game/Blueprints/Grabeable/BP_Gem.BP_Gem_C" (`KismetMathLibrary.MakeTransform` (`self.K2_GetActorLocation`)) "Undefined" "OverrideRootScale" null null)))
    (:`then_1`
      (`self.K2_DestroyActor`))))

(fn `UserConstructionScript`)