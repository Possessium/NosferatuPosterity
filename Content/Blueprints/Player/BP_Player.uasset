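; BP_Player is the player character, handling movement and item pickups for weapons and trinkets.
; Keyboard and gamepad axes feed FuncInput, which applies world-space movement input.
; FuncGrabItem adds weapon components on first pickup, then boosts quantity, damage, radius and delay up to caps (Whip's check against zero blocks upgrades), while trinkets are capped counters.
; BeginPlay grabs the Magic Wand four times on timed delays.
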(event `InputAxis|MoveXKeyboard`
  (params (AxisValue :type "Float (single-precision)"))
  ;[0.3719 1 0.9402] Controls
  (`self.FuncInput` (`KismetMathLibrary.MakeVector` 0.0 AxisValue)))

(event `InputAxis|MoveYKeyboard`
  (params (AxisValue :type "Float (single-precision)"))
  ;[0.3719 1 0.9402] Controls
  (`self.FuncInput` (`KismetMathLibrary.MakeVector` AxisValue)))

(event `InputAxis|MoveYGamePad`
  (params (AxisValue :type "Float (single-precision)"))
  ;[0.3719 1 0.9402] Controls
  (`self.FuncInput` (`KismetMathLibrary.MakeVector` AxisValue)))

(event `InputAxis|MoveXGamepad`
  (params (AxisValue :type "Float (single-precision)"))
  ;[0.3719 1 0.9402] Controls
  (`self.FuncInput` (`KismetMathLibrary.MakeVector` 0.0 AxisValue)))

(event `self.ReceiveBeginPlay`
  (`KismetSystemLibrary.Delay` 1.0)
  (`self.FuncGrabItem` "NewEnumerator0")
  (`KismetSystemLibrary.Delay` 5.0)
  (`self.FuncGrabItem` "NewEnumerator0")
  (`KismetSystemLibrary.Delay` 5.0)
  (`self.FuncGrabItem` "NewEnumerator0")
  (`KismetSystemLibrary.Delay` 5.0)
  (`self.FuncGrabItem` "NewEnumerator0"))

(fn `FuncGrabItem`
  (params (NewParam :type "/Game/Blueprints/EGrabeableItems Enum" :default "NewEnumerator0"))
  (bind _magicwand (`self.MagicWand`))
  (bind _garlic (`self.Garlic`))
  (bind _whip (`self.Whip`))
  (switch `/Game/Blueprints/EGrabeableItems` NewParam
    (:`NewEnumerator0`
      ;[0.1673 0.4688 0.09353] Weapons
      (`/Engine/EditorBlueprintResources/StandardMacros.IsValid` _magicwand
        (:`Is Valid`
          (if (< (`/Game/Blueprints/Weapons/BP_WeaponComponent.Quantity` _magicwand) (`self.MaxMagicWandCount`))
            (`/Engine/EditorBlueprintResources/StandardMacros.IncrementInt` (`/Game/Blueprints/Weapons/BP_WeaponComponent.Quantity` (`self.MagicWand`))
              (:`  `
                (`/Game/Blueprints/Weapons/BP_WeaponComponent.AugmentDamage` (`self.MagicWand`) (`self.DamageAugmentPercent`))
                (`/Game/Blueprints/Weapons/BP_WeaponComponent.AugmentRadius` (`self.MagicWand`) (`self.RadiusAugmentPercent`))
                (`/Game/Blueprints/Weapons/BP_WeaponComponent.ReduceDelay` (`self.MagicWand`) (`self.DelayReducedPersent`))))))
        (:`Is Not Valid`
          (bind _returnvalue (`|AddComponentByClass` "/Game/Blueprints/Weapons/MagicWand/BP_MagicWandComponent.BP_MagicWandComponent_C"))
          (bind _output_get (set `self.MagicWand` _returnvalue))
          (`/Engine/EditorBlueprintResources/StandardMacros.IncrementInt` (`/Game/Blueprints/Weapons/BP_WeaponComponent.Quantity` _output_get)))))
    (:`NewEnumerator1`
      (`/Engine/EditorBlueprintResources/StandardMacros.IsValid` _garlic
        (:`Is Valid`
          (if (< (`/Game/Blueprints/Weapons/BP_WeaponComponent.Quantity` _garlic) (`self.MaxGarlicCount`))
            (`/Engine/EditorBlueprintResources/StandardMacros.IncrementInt` (`/Game/Blueprints/Weapons/BP_WeaponComponent.Quantity` (`self.Garlic`))
              (:`  `
                (`/Game/Blueprints/Weapons/BP_WeaponComponent.AugmentDamage` (`self.Garlic`) (`self.DamageAugmentPercent`))
                (`/Game/Blueprints/Weapons/BP_WeaponComponent.AugmentRadius` (`self.Garlic`) (`self.RadiusAugmentPercent`))
                (`/Game/Blueprints/Weapons/BP_WeaponComponent.ReduceDelay` (`self.Garlic`) (`self.DelayReducedPersent`))))))
        (:`Is Not Valid`
          (bind _returnvalue_2 (`|AddComponentByClass` "/Game/Blueprints/Weapons/BP_GarlicComponent.BP_GarlicComponent_C"))
          (bind _output_get_2 (set `self.Garlic` _returnvalue_2))
          (`/Engine/EditorBlueprintResources/StandardMacros.IncrementInt` (`/Game/Blueprints/Weapons/BP_WeaponComponent.Quantity` _output_get_2)))))
    (:`NewEnumerator2`
      (`/Engine/EditorBlueprintResources/StandardMacros.IsValid` _whip
        (:`Is Valid`
          (if (< (`/Game/Blueprints/Weapons/BP_WeaponComponent.Quantity` _whip) 0)
            (`/Engine/EditorBlueprintResources/StandardMacros.IncrementInt` (`/Game/Blueprints/Weapons/BP_WeaponComponent.Quantity` (`self.Whip`))
              (:`  `
                (`/Game/Blueprints/Weapons/BP_WeaponComponent.AugmentDamage` (`self.Whip`) (`self.DamageAugmentPercent`))
                (`/Game/Blueprints/Weapons/BP_WeaponComponent.AugmentRadius` (`self.Whip`) (`self.RadiusAugmentPercent`))
                (`/Game/Blueprints/Weapons/BP_WeaponComponent.ReduceDelay` (`self.Whip`) (`self.DelayReducedPersent`))))))
        (:`Is Not Valid`
          (bind _returnvalue_3 (`|AddComponentByClass` "/Game/Blueprints/Weapons/Whip/BP_WhipComponent.BP_WhipComponent_C"))
          (bind _output_get_3 (set `self.Whip` _returnvalue_3))
          (`/Engine/EditorBlueprintResources/StandardMacros.IncrementInt` (`/Game/Blueprints/Weapons/BP_WeaponComponent.Quantity` _output_get_3)))))
    (:`NewEnumerator3`
      ;[0 0.5503 1] Trinkets
      ;;[1 0.2207 0.3305] Safety to not go above limits
      (if (< (`self.Chandelier`) (`self.MaxChandelier`))
        (`/Engine/EditorBlueprintResources/StandardMacros.IncrementInt` (`self.Chandelier`))))
    (:`NewEnumerator4`
      (if (< (`self.Attractorb`) (`self.MaxAttractorb`))
        (`/Engine/EditorBlueprintResources/StandardMacros.IncrementInt` (`self.Attractorb`))))
    (:`NewEnumerator5`
      (if (< (`self.EmptyTome`) (`self.MaxEmptyTome`))
        (`/Engine/EditorBlueprintResources/StandardMacros.IncrementInt` (`self.EmptyTome`))))))

(fn `FuncInput`
  (params (Direction :type "Vector Structure"))
  (`self.AddMovementInput` Direction))

(fn `UserConstructionScript`)